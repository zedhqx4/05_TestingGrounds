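; AI controller for guard NPCs that runs the GuardBehaviour behavior tree on the PatrolData blackboard.
; AI perception updates write a sensed actor to the blackboard enemy key and clear it on a failed sense, ignoring actors tagged Guard.
; Each tick, the controlled Character aims and shoots whenever the controller has a valid focus actor; this file's live logic never sets that focus itself.
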(event OnTargetPerceptionUpdated(AIPerception)
  (params (Actor :type Actor%20Object%20Reference) (Stimulus :type AI%20Stimulus%20Structure))
  ;[1 1 1] Comment
  (CallFunction|UpdateBlackboardEnemyKey Actor Stimulus Actor))

(event EventBeginPlay
  ;[1 1 1] Begin Play
  (bind _blackboardcomponent (Class|AIController|UseBlackboard "/Game/Dynamic/Character/AI/PatrolData.PatrolData"))
  (AI|RunBehaviorTree "/Game/Dynamic/Character/AI/GuardBehaviour.GuardBehaviour")
  (Variables|Default|SetBlackboardComp _blackboardcomponent))

(event EventTick
  (params (DeltaSeconds :type Float%20%28single-precision%29))
  ;[1 1 1] Set aiming
  (bind _ascharacter (Utilities|Casting|CastToCharacter (Pawn|GetControlledPawn)))
  (bind _output_get (Variables|/Game/Dynamic/Character/Behaviour/Character.Character_C|SetAimingCharacter _ascharacter (Utilities|IsValid (Class|AIController|GetFocusActor))))
  (Variables|/Game/Dynamic/Character/Behaviour/Character.Character_C|SetShootingCharacter _ascharacter _output_get))

(fn ConstructionScript)

(fn UpdateBlackboardEnemyKey
  (params (ObjectValue :type Object%20Object%20Reference) (AIStimulus :type AI%20Stimulus%20Structure%20%28by%20ref%29) (self2 :type Actor%20Object%20Reference))
  (bind _enemykey (Variables|Default|GetEnemyKey))
  (bind _blackboardcomp (Variables|Default|GetBlackboardComp))
  (if (not (Actor|ActorHasTag self2 "Guard"))
    (if (.bSuccessfullySensed (Utilities|Struct|BreakAIStimulus AIStimulus))
      (AI|Components|Blackboard|SetValueasObject _blackboardcomp _enemykey ObjectValue)
      (else
        (AI|Components|Blackboard|ClearValue _blackboardcomp _enemykey)))))